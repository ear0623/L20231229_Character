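; Blue warp visual effect actor built from layered meshes and a Stars particle component, configured entirely in the construction script.
; It passes an acceleration vector to the stars and creates dynamic materials for the background, sphere, intensive and main warp meshes.
; Exposed speed and color variables drive the warp layers, while the background color gets a random RGB offset on every construction run.
; The event graph has no active logic.
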(event EventBeginPlay)

(event Collision|EventActorBeginOverlap
  (params (OtherActor :type Actor%20Object%20Reference)))

(event EventTick
  (params (DeltaSeconds :type Float%20%28single-precision%29)))

(fn ConstructionScript
  (bind _sm_warpmain (Variables|Default|GetSM_WarpMain))
  (bind _sm_warpintensive (Variables|Default|GetSM_WarpIntensive))
  (bind _sm_warpbg (Variables|Default|GetSM_WarpBG))
  (bind _sphere (Variables|Default|GetSphere))
  (bind _sm_warpmain_2 (Variables|Default|GetSM_WarpMain))
  (Effects|Components|ParticleSystem|SetVectorParameter (Variables|Default|GetStars) "Acc" (Variables|Default|GetParticle%20acceleration))
  (Rendering|Material|CreateDynamicMaterialInstance _sm_warpbg 0 (Rendering|Material|GetMaterial _sm_warpbg 0) "None" :!class /Script/Engine.PrimitiveComponent)
  (Variables|Default|SetColor_BG (+ (Variables|Default|GetColor_BG) (Utilities|Struct|MakeLinearColor (Math|Random|RandomFloatinRange 0.0 1.0) (Math|Random|RandomFloatinRange 0.0 1.0) (Math|Random|RandomFloatinRange 0.0 1.0) 1.0)))
  (Rendering|Material|SetVectorParameterValueonMaterials _sm_warpbg "Color" (Math|Conversions|ToVector(LinearColor) (Variables|Default|GetColor_BG)))
  (Rendering|Material|CreateDynamicMaterialInstance _sphere 0 (Rendering|Material|GetMaterial _sphere 0) "None" :!class /Script/Engine.PrimitiveComponent)
  (Rendering|Material|SetScalarParameterValueonMaterials _sphere "Speed" (Variables|Default|GetSpeed))
  (Rendering|Material|SetVectorParameterValueonMaterials _sphere "Color_Tex1" (Math|Conversions|ToVector(LinearColor) (Variables|Default|GetColor_4)))
  (Rendering|Material|CreateDynamicMaterialInstance _sm_warpintensive 0 (Rendering|Material|GetMaterial _sm_warpintensive 0) "None" :!class /Script/Engine.PrimitiveComponent)
  (Rendering|Material|SetVectorParameterValueonMaterials _sm_warpintensive "Color_Tex1" (Math|Conversions|ToVector(LinearColor) (Variables|Default|GetColor_4)))
  (Rendering|Material|SetScalarParameterValueonMaterials (Variables|Default|GetSM_WarpIntensive) "Speed" (Variables|Default|GetSpeed))
  (bind _returnvalue (Rendering|Material|CreateDynamicMaterialInstance _sm_warpmain 0 (Rendering|Material|GetMaterial _sm_warpmain 0) "None" :!class /Script/Engine.PrimitiveComponent))
  (Rendering|Material|SetScalarParameterValue _returnvalue "Speed" (Variables|Default|GetSpeed) :!class /Script/Engine.MaterialInstanceDynamic)
  (Rendering|Material|SetVectorParameterValueonMaterials _sm_warpmain_2 "Color_Tex1" (Math|Conversions|ToVector(LinearColor) (Variables|Default|GetColor_1)))
  (Rendering|Material|SetVectorParameterValueonMaterials _sm_warpmain_2 "Color_Tex2" (Math|Conversions|ToVector(LinearColor) (Variables|Default|GetColor_2)))
  (Rendering|Material|SetVectorParameterValueonMaterials _sm_warpmain_2 "Color_Tex3" (Math|Conversions|ToVector(LinearColor) (Variables|Default|GetColor_3))))