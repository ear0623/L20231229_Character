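; BP_Earth2 is a spinning globe actor that plots latitude/longitude points from the SircleData table as mesh instances on a sphere.
; The construction script converts rows to Cartesian positions at PlanSize radius, with Z negated, and adds them to a hierarchical instanced static mesh.
; It loops over a fixed index range rather than the table's row count.
; A looping timer from BeginPlay rotates the scene root in fixed steps, without using Tick.
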(event EventBeginPlay
  (Utilities|Time|SetTimerbyFunctionName 0 "UpdateRotate" 0.1 true))

(event Collision|EventActorBeginOverlap
  (params (OtherActor :type Actor%20Object%20Reference)))

(event EventTick
  (params (DeltaSeconds :type Float%20%28single-precision%29)))

(fn ConstructionScript
  (bind _plansize (Variables|Default|GetPlanSize))
  (bind _outrownames (DataTable|GetDataTableRowNames "/Game/EarthMaterials/SircleData.SircleData"))
  (for _index (range 0 1000)
    (bind _returnvalue (Utilities|GetDataTableRow "/Game/EarthMaterials/SircleData.SircleData" (Utilities|Array|Get(acopy) _outrownames _index))
      (:then
        (bind _output_get (Variables|Default|SetArray (Utilities|Array|MakeArray (Math|Transform|MakeTransform (Math|Vector|MakeVector (* _plansize (* (Math|Trig|Cos(Degrees) (.lat _returnvalue)) (Math|Trig|Cos(Degrees) (.lng _returnvalue)))) (* _plansize (* (Math|Trig|Cos(Degrees) (.lat _returnvalue)) (Math|Trig|Sin(Degrees) (.lng _returnvalue)))) (* (* _plansize -1.0) (Math|Trig|Sin(Degrees) (.lat _returnvalue))))))))
        (Components|InstancedStaticMesh|AddInstances (Variables|Default|GetHierarchicalInstancedStaticMesh) _output_get false false)))))

(fn UpdateRotate
  (Transformation|AddLocalRotation (Variables|Default|GetDefaultSceneRoot) "0.000000,0.000000,10.000000" false false))