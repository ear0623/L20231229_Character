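; BP_Earth is an Actor Blueprint that places an instance for each city in the Worldcities data table around an Earth of radius PlanSize.
; The construction script converts each row's latitude and longitude to Cartesian offsets and adds them to a HierarchicalInstancedStaticMesh.
; Z uses the sine of longitude rather than latitude, so points deviate from a true spherical mapping.
; The event graph holds only disabled placeholder events.
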(event EventBeginPlay)

(event Collision|EventActorBeginOverlap
  (params (OtherActor :type Actor%20Object%20Reference)))

(event EventTick
  (params (DeltaSeconds :type Float%20%28single-precision%29)))

(fn ConstructionScript
  (bind _plansize (Variables|Default|GetPlanSize))
  (bind _outrownames (DataTable|GetDataTableRowNames "/Game/EarthMaterials/worldcities.worldcities"))
  (for _index (range 0 (Utilities|Array|Length _outrownames))
    (bind _returnvalue (Utilities|GetDataTableRow "/Game/EarthMaterials/worldcities.worldcities" (Utilities|Array|Get(acopy) _outrownames _index))
      (:then
        (Components|InstancedStaticMesh|AddInstance (Variables|Default|GetHierarchicalInstancedStaticMesh) (Math|Transform|MakeTransform (Math|Vector|MakeVector (* _plansize (* (Math|Trig|Cos(Degrees) (.lat _returnvalue)) (Math|Trig|Cos(Degrees) (.lng _returnvalue)))) (* _plansize (* (Math|Trig|Cos(Degrees) (.lat _returnvalue)) (Math|Trig|Sin(Degrees) (.lng _returnvalue)))) (* _plansize (Math|Trig|Sin(Degrees) (.lng _returnvalue)))) "0, 0, 0" "1.000000,1.000000,1.000000") false)))))