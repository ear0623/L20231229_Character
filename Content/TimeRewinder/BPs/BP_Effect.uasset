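; BP_Effect is a test effect actor in TimeRewinder that repeatedly spawns an explosion with audio.
; Tick feeds a self-looping two-second Delay that spawns P_Explosion at the actor's transform and plays the Audio component.
; Each pass offsets and negates StartTime before playback, then prints the negated result of GetPlayLengthMessage.
; The playback-percent binding is unconnected and its handler is empty.
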(event Custom|OnAudioPlaybackPercent_Event
  (params (PlayingSoundWave :type Sound%20Wave%20Object%20Reference) (PlaybackPercent :type Float%20%28single-precision%29)))

(event EventBeginPlay)

(event Collision|EventActorBeginOverlap
  (params (OtherActor :type Actor%20Object%20Reference)))

(event EventTick
  (params (DeltaSeconds :type Float%20%28single-precision%29))
  (bind _self self)
  (bind _returnvalue (Transformation|GetActorTransform _self))
  (Utilities|FlowControl|Delay 2.0)
  (Effects|SpawnEmitteratLocation "/Game/StarterContent/Particles/P_Explosion.P_Explosion" (.location _returnvalue) (.rotation _returnvalue) (.scale _returnvalue) :!label _label)
  (Variables|Default|SetStart%20Time (* (+ (Variables|Default|GetStart%20Time) 0.1) -1.0))
  (Audio|Components|Audio|Play (Variables|Default|GetAudio) (Variables|Default|GetStart%20Time))
  (bind _returnvalue_2 (Animation|GetPlayLength (Variables|Default|GetAudio)))
  (Development|PrintString (Utilities|String|ToString(Float) (* _returnvalue_2 -1.0)))
  (Utilities|FlowControl|Delay 2.0)
  (goto _label))

(fn ConstructionScript)